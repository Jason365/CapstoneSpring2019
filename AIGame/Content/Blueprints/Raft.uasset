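; Raft actor that rides the height of the surface at its position, presumably water.
; Each tick it line-traces vertically through its location on a custom channel, with debug drawing on, and does a swept move to slightly above the hit, keeping X and Y.
; The hit result is not checked before use.
; BeginPlay caches the first WaterLayer actor, but the tick logic never uses it.
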(event `self.ReceiveBeginPlay`
  (bind _outactors (`GameplayStatics.GetAllActorsOfClass` "/Game/Blueprints/WaterLayer.WaterLayer_C"))
  (set `self.Water` (`|GetArrayItem` _outactors)))

(event `self.ReceiveTick`
  (params (DeltaSeconds :type "Float (single-precision)"))
  (bind _returnvalue (`self.K2_GetActorLocation`))
  (bind (_returnvalue_x _returnvalue_y) (`KismetMathLibrary.BreakVector` (`self.K2_GetActorLocation`)))
  (bind _outhit (`KismetSystemLibrary.LineTraceSingle` :`Start` (`KismetMathLibrary.MakeVector` (.x _returnvalue) (.y _returnvalue) (+ (.z _returnvalue) 500.0)) :`End` (`KismetMathLibrary.MakeVector` (.x _returnvalue) (.y _returnvalue) (- (.z _returnvalue) 500.0)) :`TraceChannel` "TraceTypeQuery4" :`DrawDebugType` "ForOneFrame"))
  (`self.K2_SetActorLocation` (`KismetMathLibrary.MakeVector` _returnvalue_x _returnvalue_y (+ (.z (`.Location` (`GameplayStatics.BreakHitResult` _outhit))) 30.0)) true))

(fn `UserConstructionScript`)