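; TreeDestroyer is an actor Blueprint that randomly thins out the Tree actors in the level when play begins.
; On BeginPlay it gathers all Tree actors and makes random picks, with the pick count based on a random fraction of the total.
; Picks go into ToRemove through AddUnique, so repeats collapse and fewer trees may be removed.
; A second loop then destroys every collected tree.
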(event `self.ReceiveBeginPlay`
  (bind _toremove (`self.toRemove`))
  (bind _outactors (`GameplayStatics.GetAllActorsOfClass` "/Game/Inventory/Destructibles/Tree.Tree_C"))
  (bind _returnvalue (`KismetArrayLibrary.Array_Length` _outactors))
  (for _ (range (+ (`KismetMathLibrary.FTrunc` (* _returnvalue (`KismetMathLibrary.RandomFloatInRange` 0.15 0.3))) 1))
    (`KismetArrayLibrary.Array_AddUnique` _toremove (`|GetArrayItem` _outactors (`KismetMathLibrary.RandomIntegerInRange` 0 (- _returnvalue 1)))))
  (for _array_element _toremove
    (`self.K2_DestroyActor` _array_element)))

(fn `UserConstructionScript`)